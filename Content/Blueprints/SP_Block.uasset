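; SP_Block is a hittable block actor that awards a coin and plays a bump animation.
; A box component hit, when the block is enabled, disables it and calls EventGetCoin on SP_GameMode.
; A timeline then offsets the block vertically from its BeginPlay location and swaps the cube material to a concrete floor.
; Actor overlap sets the enabled flag, and BreakBlock is an empty stub.
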(event `self.ReceiveBeginPlay`
  (set `self.startLocation` (`SceneComponent.K2_GetComponentLocation` (`self.DefaultSceneRoot`))))

(event `self.ReceiveActorBeginOverlap`
  (params (OtherActor :type "Actor Object Reference"))
  (set `self.isEnabled` true))

(event `self.Box.OnComponentHit`
  (params (HitComponent :type "PrimitiveComponent Object Reference") (OtherActor :type "Actor Object Reference") (OtherComp :type "PrimitiveComponent Object Reference") (NormalImpulse :type "Vector Structure") (Hit :type "HitResult Structure (by ref)"))
  (if (`self.isEnabled`)
    (set `self.isEnabled` false)
    (bind _assp_game_mode (cast `/Game/SP_GameMode` (`GameplayStatics.GetGameMode`)))
    (`/Game/SP_GameMode.Event GetCoin` _assp_game_mode)
    (bind (_direction _updown) (`Timeline|Timeline_0`)
      (:`Update`
        (`PrimitiveComponent.SetMaterial` (`self.Cube`) 0 "/Game/SoulCity/Environment/Materials/Building/MI_Slums_Concrete_002_Floor.MI_Slums_Concrete_002_Floor")
        (`SceneComponent.K2_SetWorldLocation` (`self.DefaultSceneRoot`) (+ (`KismetMathLibrary.MakeVector` 0.0 0.0 _updown) (`self.startLocation`)) false false)))))

(fn `breakBlock`)

(fn `UserConstructionScript`)