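; Base portal actor that teleports whatever is passed to its Interaction function to the location of its linked target portal.
; On BeginPlay it records its start location and, if the target portal is already initialized, the two exchange locations, so linking works in both directions.
; Trigger overlap plays a swoosh, shows Info and moves the portal vertically with the Down timeline, while end overlap hides Info and plays Up.
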(event `InitTargetPortal`
  (params (targetPotal :type "/Game/Blueprints/SP_BasePortal Object Reference"))
  (if (`/Game/Blueprints/SP_BasePortal.isCreated` targetPotal)
    (bind _output_get (set `self.targetLocation` (`/Game/Blueprints/SP_BasePortal.startLocation` targetPotal)))
    (set `/Game/Blueprints/SP_BasePortal.targetLocation` (`self.startLocation`) targetPotal)
    (`KismetSystemLibrary.PrintString` (`KismetStringLibrary.Concat_StrStr` "targetLocation : " (`KismetStringLibrary.Conv_VectorToString` _output_get)))))

(event `self.ReceiveBeginPlay`
  (bind _output_get (set `self.startLocation` (`SceneComponent.K2_GetComponentLocation` (`self.DefaultSceneRoot`))))
  (`KismetSystemLibrary.PrintString` (`KismetStringLibrary.Concat_StrStr` "StartLocation : " (`KismetStringLibrary.Conv_VectorToString` _output_get)))
  (set `self.isCreated` true)
  (`self.InitTargetPortal` (`self.targetPortal`)))

(event `self.Trigger.OnComponentBeginOverlap`
  (params (OverlappedComponent :type "PrimitiveComponent Object Reference") (OtherActor :type "Actor Object Reference") (OtherComp :type "PrimitiveComponent Object Reference") (OtherBodyIndex :type Integer) (bFromSweep :type Boolean) (SweepResult :type "HitResult Structure (by ref)"))
  (if (not (`self.isOn`))
    (set `self.isOn` true)
    (`GameplayStatics.PlaySoundAtLocation` "/Game/sound/Swoosh.Swoosh" (`self.startLocation`) (struct) 1.0 1.0 0.0 null null null)
    (`SceneComponent.SetVisibility` (`self.Info`) true false)
    (bind (_direction _down) (`Timeline|Down`)
      (:`Update`
        (`SceneComponent.K2_SetWorldLocation` (`self.DefaultSceneRoot`) (+ (`KismetMathLibrary.MakeVector` 0.0 0.0 _down) (`self.startLocation`)) false false)))))

(event `self.Trigger.OnComponentEndOverlap`
  (params (OverlappedComponent :type "PrimitiveComponent Object Reference") (OtherActor :type "Actor Object Reference") (OtherComp :type "PrimitiveComponent Object Reference") (OtherBodyIndex :type Integer))
  (if (`self.isOn`)
    (set `self.isOn` false)
    (`SceneComponent.SetVisibility` (`self.Info`) false false)
    (bind (_direction _up) (`Timeline|Up`)
      (:`Update`
        (`SceneComponent.K2_SetWorldLocation` (`self.DefaultSceneRoot`) (+ (`KismetMathLibrary.MakeVector` 0.0 0.0 _up) (`self.startLocation`)) false false)))))

(fn `Interaction`
  (params (phase :type "/Game/Character/SP_Phase Object Reference"))
  (returns (isSucceeded :type Boolean))
  (`/Game/Character/SP_Phase.Teleport` phase (`self.targetLocation`))
  (return true))

(fn `UserConstructionScript`)